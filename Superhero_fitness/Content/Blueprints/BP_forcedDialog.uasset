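; BP_forcedDialog plays a one-time opening conversation that the player must click through before playing.
; On BeginPlay, if the game instance has not marked it as played, it shows a Forced_dialog widget and moves input from the pawn to itself.
; Each Space press feeds the next InitalConversation line to the widget.
; After the last line, it restores pawn input, hides the widget and sets PlayedInitalDialog on BP_playerInstacne.
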(event `self.ReceiveBeginPlay`
  (bind _returnvalue (`GameplayStatics.GetPlayerController` 0))
  (bind _asbp_player_instacne (cast `/Game/Blueprints/BP_playerInstacne` (`GameplayStatics.GetGameInstance`)))
  (if (not (`/Game/Blueprints/BP_playerInstacne.PlayedInitalDialog?` _asbp_player_instacne))
    (bind _returnvalue_2 (`|CreateWidget` "/Game/UI/DialogUI/Forced_dialog.Forced_dialog_C"))
    (`UserWidget.AddToViewport` _returnvalue_2 0)
    (set `self.TalkingUI` _returnvalue_2)
    (`self.EnableInput` _returnvalue)
    (`self.DisableInput` (`GameplayStatics.GetPlayerPawn` 0) _returnvalue)))

(event `Key|SpaceBar`
  (params (Key :type "Key Structure"))
  (bind _returnvalue (`GameplayStatics.GetPlayerController` 0))
  (:`Pressed`
    (if (>= (`self.TalkingIndex`) (`KismetArrayLibrary.Array_Length` (`self.Inital_Conversation`)))
      (`self.EnableInput` (`GameplayStatics.GetPlayerPawn` 0) _returnvalue)
      (`self.DisableInput` _returnvalue)
      (`Widget.SetVisibility` (`self.TalkingUI`) "Hidden")
      (bind _asbp_player_instacne (cast `/Game/Blueprints/BP_playerInstacne` (`GameplayStatics.GetGameInstance`)))
      (set `/Game/Blueprints/BP_playerInstacne.PlayedInitalDialog?` true _asbp_player_instacne)
      (else
        (`/Game/UI/DialogUI/Forced_dialog.ProgessConversation` (`self.TalkingUI`) (`|GetArrayItem` (`self.Inital_Conversation`) (`self.TalkingIndex`)))
        (set `self.TalkingIndex` (+ (`self.TalkingIndex`) 1))))))

(fn `UserConstructionScript`)