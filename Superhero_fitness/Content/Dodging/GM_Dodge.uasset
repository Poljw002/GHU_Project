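; GM_Dodge is the game mode for a dodging game, keeping a Points score that rewards avoiding hits.
; BeginPlay adds the Counter_Dodge widget to the viewport.
; Tick polls the hero character's HasBeenHit flag, deducting points and clearing it on a hit.
; Otherwise a latent Delay in Tick throttles the reward to roughly one award per second.
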(event `self.ReceiveBeginPlay`
  (bind _returnvalue (`|CreateWidget` "/Game/Dodging/Counter_Dodge.Counter_Dodge_C"))
  (`UserWidget.AddToViewport` _returnvalue 0))

(event `self.ReceiveTick`
  (params (DeltaSeconds :type "Float (single-precision)"))
  (bind _asbp_third_person_character_hero (cast `/Game/ThirdPerson/Blueprints/BP_ThirdPersonCharacter_hero` (`GameplayStatics.GetPlayerPawn` 0)))
  (if (`/Game/ThirdPerson/Blueprints/BP_ThirdPersonCharacter_hero.HasBeenHit` _asbp_third_person_character_hero)
    (set `self.Points` (- (`self.Points`) 10.0))
    (set `/Game/ThirdPerson/Blueprints/BP_ThirdPersonCharacter_hero.HasBeenHit` false _asbp_third_person_character_hero)
    (else
      (`KismetSystemLibrary.Delay` 1.0)
      (set `self.Points` (+ (`self.Points`) 5.0)))))

(fn `UserConstructionScript`)