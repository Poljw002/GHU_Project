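; Diet minigame lane that sends out random healthy or junk food for the player to eat with a timed Space press.
; SpawnNewFeed, gated by Playing, spawns and moves one item, replaced when bitten or when it hits the Destroyer.
; Tick polls the Sphere's overlaps by food class to set Overlapping and IsHealthy.
; A bite plays a sound, clears the Sphere and adjusts Points and the game instance's MindStat: up for healthy, down for junk.
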(event `self.ReceiveBeginPlay`
  (`self.EnableInput` (`GameplayStatics.GetPlayerController` 0))
  (`self.Spawn new feed` :!label _label))

(event `self.Destroyer.OnComponentBeginOverlap`
  (params (OverlappedComponent :type "PrimitiveComponent Object Reference") (OtherActor :type "Actor Object Reference") (OtherComp :type "PrimitiveComponent Object Reference") (OtherBodyIndex :type Integer) (bFromSweep :type Boolean) (SweepResult :type "HitResult Structure (by ref)"))
  (`self.K2_DestroyActor` OtherActor)
  (goto _label))

(event `Key|SpaceBar`
  (params (Key :type "Key Structure"))
  (:`Pressed`
    (if (`self.Overlapping`)
      (`|ExecutionSequence`
        (:`then_0`
          (`GameplayStatics.PlaySound2D` "/Game/DietFolder/Bite.Bite" 1.0 1.0 0.0 null null))
        (:`then_1`
          (`|ExecutionSequence`
            (:`then_0`
              (`|ExecutionSequence`
                (:`then_0`
                  (bind _asbp_player_instacne (cast `/Game/Blueprints/BP_playerInstacne` (`GameplayStatics.GetGameInstance`)))
                  (set `self.As BP Player Instacne` _asbp_player_instacne))
                (:`then_1`
                  (`|ExecutionSequence`
                    (:`then_0`
                      (if (`self.IsHealthy`)
                        (set `self.Points` (+ 2.0 (`self.Points`)))
                        (else
                          (set `self.Points` (- (`self.Points`) 1.0)))))
                    (:`then_1`
                      (if (`self.IsHealthy`)
                        (set `/Game/Blueprints/BP_playerInstacne.mind_stat` (+ (`/Game/Blueprints/BP_playerInstacne.mind_stat` (`self.As BP Player Instacne`)) 2.0) (`self.As BP Player Instacne`))
                        (else
                          (set `/Game/Blueprints/BP_playerInstacne.mind_stat` (- (`/Game/Blueprints/BP_playerInstacne.mind_stat` (`self.As BP Player Instacne`)) 1.0) (`self.As BP Player Instacne`)))))))))
            (:`then_1`
              (`self.K2_DestroyActor` (`PrimitiveComponent.GetOverlappingActors` (`self.Sphere`) "/Game/DietFolder/FoodsBP/BP_Cake.BP_Cake_C")))
            (:`then_2`
              (`self.K2_DestroyActor` (`PrimitiveComponent.GetOverlappingActors` (`self.Sphere`) "/Game/DietFolder/FoodsBP/BP_Donut.BP_Donut_C")))
            (:`then_3`
              (`self.K2_DestroyActor` (`PrimitiveComponent.GetOverlappingActors` (`self.Sphere`) "/Game/DietFolder/FoodsBP/BP_Carrot.BP_Carrot_C")))
            (:`then_4`
              (`self.K2_DestroyActor` (`PrimitiveComponent.GetOverlappingActors` (`self.Sphere`) "/Game/DietFolder/FoodsBP/BP_GreenApple.BP_GreenApple_C")))
            (:`then_5`
              (`self.K2_DestroyActor` (`PrimitiveComponent.GetOverlappingActors` (`self.Sphere`) "/Game/DietFolder/FoodsBP/BP_RedApple.BP_RedApple_C")))
            (:`then_6`
              (`self.K2_DestroyActor` (`PrimitiveComponent.GetOverlappingActors` (`self.Sphere`) "/Game/DietFolder/FoodsBP/BP_Strawberry.BP_Strawberry_C")))
            (:`then_7`
              (`self.Spawn new feed`)))))
      (else
        (`KismetSystemLibrary.PrintString` "Miss")))))

(event `self.ReceiveTick`
  (params (DeltaSeconds :type "Float (single-precision)"))
  (bind _returnvalue (!= (`KismetArrayLibrary.Array_Length` (`PrimitiveComponent.GetOverlappingActors` (`self.Sphere`) "/Game/DietFolder/FoodsBP/BP_Cake.BP_Cake_C")) 0))
  (bind _returnvalue_2 (!= (`KismetArrayLibrary.Array_Length` (`PrimitiveComponent.GetOverlappingActors` (`self.Sphere`) "/Game/DietFolder/FoodsBP/BP_Donut.BP_Donut_C")) 0))
  (if (or _returnvalue (!= (`KismetArrayLibrary.Array_Length` (`PrimitiveComponent.GetOverlappingActors` (`self.Sphere`) "/Game/DietFolder/FoodsBP/BP_Carrot.BP_Carrot_C")) 0) _returnvalue_2 (!= (`KismetArrayLibrary.Array_Length` (`PrimitiveComponent.GetOverlappingActors` (`self.Sphere`) "/Game/DietFolder/FoodsBP/BP_GreenApple.BP_GreenApple_C")) 0) (!= (`KismetArrayLibrary.Array_Length` (`PrimitiveComponent.GetOverlappingActors` (`self.Sphere`) "/Game/DietFolder/FoodsBP/BP_RedApple.BP_RedApple_C")) 0) (!= (`KismetArrayLibrary.Array_Length` (`PrimitiveComponent.GetOverlappingActors` (`self.Sphere`) "/Game/DietFolder/FoodsBP/BP_Strawberry.BP_Strawberry_C")) 0))
    (set `self.Overlapping` true)
    (if (or _returnvalue _returnvalue_2)
      (set `self.IsHealthy` false)
      (else
        (set `self.IsHealthy` true)))
    (else
      (set `self.Overlapping` false))))

(fn `Spawn new feed`
  (bind _returnvalue (`KismetMathLibrary.RandomInteger` 4))
  (if (`self.playing`)
    (if (!= (`KismetMathLibrary.RandomInteger` 2) 1)
      (if (== _returnvalue 0)
        (bind _returnvalue_2 (`|SpawnActorFromClass` "/Game/DietFolder/FoodsBP/BP_Strawberry.BP_Strawberry_C" (`KismetMathLibrary.MakeTransform` (0.0 0.0 0.0) (struct) (10.0 10.0 10.0)) "Undefined" "MultiplyWithRoot" null null))
        (`/Game/DietFolder/FoodsBP/BP_Strawberry.Move Food` _returnvalue_2)
        (elif (== _returnvalue 1)
          (bind _returnvalue_3 (`|SpawnActorFromClass` "/Game/DietFolder/FoodsBP/BP_Carrot.BP_Carrot_C" (`KismetMathLibrary.MakeTransform` (0.0 0.0 0.0) (struct) (10.0 10.0 10.0)) "Undefined" "MultiplyWithRoot" null null))
          (`/Game/DietFolder/FoodsBP/BP_Carrot.Move Food` _returnvalue_3)
          (elif (== _returnvalue 2)
            (bind _returnvalue_4 (`|SpawnActorFromClass` "/Game/DietFolder/FoodsBP/BP_GreenApple.BP_GreenApple_C" (`KismetMathLibrary.MakeTransform` (0.0 0.0 0.0) (struct) (10.0 10.0 10.0)) "Undefined" "MultiplyWithRoot" null null))
            (`/Game/DietFolder/FoodsBP/BP_GreenApple.Move Food` _returnvalue_4)
            (else
              (bind _returnvalue_5 (`|SpawnActorFromClass` "/Game/DietFolder/FoodsBP/BP_RedApple.BP_RedApple_C" (`KismetMathLibrary.MakeTransform` (0.0 0.0 0.0) (struct) (10.0 10.0 10.0)) "Undefined" "MultiplyWithRoot" null null))
              (`/Game/DietFolder/FoodsBP/BP_RedApple.Move Food` _returnvalue_5)))))
      (elif (== (`KismetMathLibrary.RandomInteger` 2) 1)
        (bind _returnvalue_6 (`|SpawnActorFromClass` "/Game/DietFolder/FoodsBP/BP_Donut.BP_Donut_C" (`KismetMathLibrary.MakeTransform` (0.0 0.0 0.0) (struct) (10.0 10.0 10.0)) "Undefined" "MultiplyWithRoot" null null))
        (`/Game/DietFolder/FoodsBP/BP_Donut.Move Food` _returnvalue_6)
        (else
          (bind _returnvalue_7 (`|SpawnActorFromClass` "/Game/DietFolder/FoodsBP/BP_Cake.BP_Cake_C" (`KismetMathLibrary.MakeTransform` (0.0 0.0 0.0) (struct) (10.0 10.0 10.0)) "Undefined" "MultiplyWithRoot" null null))
          (`/Game/DietFolder/FoodsBP/BP_Cake.Move Food` _returnvalue_7))))))

(fn `UserConstructionScript`)