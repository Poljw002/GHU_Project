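; BP_Donut is a donut food actor in the diet game that travels along a lane's spline.
; On BeginPlay it caches the first BP_lane actor it finds as DietSpline.
; MoveFood plays a timeline at a rate of 1/CompletionTime, lerping distance over the spline's length to set the actor's transform.
; Only location is sampled, in spline-local space; the spline rotation lookup is left unconnected.
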(event `self.ReceiveBeginPlay`
  (bind _returnvalue (`GameplayStatics.GetActorOfClass` "/Game/DietFolder/BP_lane.BP_lane_C"))
  (set `self.Diet_Spline` _returnvalue))

(event `Move Food`
  (`TimelineComponent.SetPlayRate` (`self.Timeline`) (/ 1.0 (`self.CompletionTime`)))
  (bind (_direction _newtrack_0) (`Timeline|Timeline` :!via `PlayFromStart`)
    (:`Update`
      (`self.K2_SetActorTransform` (`KismetMathLibrary.MakeTransform` (`SplineComponent.GetLocationAtDistanceAlongSpline` (`/Game/DietFolder/BP_lane.Spline` (`self.Diet_Spline`)) (`KismetMathLibrary.Lerp` 0.0 (`SplineComponent.GetSplineLength` (`/Game/DietFolder/BP_lane.Spline` (`self.Diet_Spline`))) _newtrack_0) "Local"))))))

(fn `UserConstructionScript`)